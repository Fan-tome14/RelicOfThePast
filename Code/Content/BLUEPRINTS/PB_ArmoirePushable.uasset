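; Pushable armoire that the player shoves in axis-snapped steps, though only a pawn tagged Robot actually moves it.
; A head-on hit runs CanPush, using a line trace to confirm the target and a box trace for clearance, then locks and attaches the player and plays the push montage.
; A timeline drives each step and repeats while Z is held, without rechecking clearance, before the montage's End section releases the player.
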(event Custom|Push
  (if (Actor|ActorHasTag (Game|Player|GetPlayerPawn 0) "Robot")
    (Variables|Default|SetCurrentLocation (Transformation|GetActorLocation))
    (bind _position (Timeline|MoveBlock PlayFromStart)
      (:Update
        (Transformation|SetActorRelativeLocation (+ (Variables|Default|GetCurrentLocation) (* _position (Variables|Default|GetPushableDirection) (Variables|Default|GetTravelDistance)))))
      (:Finished
        (if (Game|Player|IsInputKeyDown (Game|GetPlayerController 0) "Z")
          (CallFunction|Push)
          (else
            (CallFunction|StopPushing)))))
    (else
      (Variables|Default|SetCurrentLocation (Transformation|GetActorLocation))
      (Timeline|PeutPasBougerBlock PlayFromStart
        (:Finished
          (if (Game|Player|IsInputKeyDown (Game|GetPlayerController 0) "Z")
            (CallFunction|Push)
            (else
              (CallFunction|StopPushing))))))))

(event Custom|StopPushing
  (bind _returnvalue (Game|GetPlayerCharacter 0))
  (Animation|Montage|PlayMontage (Variables|/Script/Engine.Character|GetMesh (Game|GetPlayerCharacter 0)) "/Game/FreeSampleAnimationSet/Animations/PushSet/RootMotion/Heavy/01/MontagePush.MontagePush" 1.0 0.0 "End"
    (:OnCompleted
      (Pawn|Components|CharacterMovement|SetMovementMode (Variables|/Script/Engine.Character|GetCharacterMovement _returnvalue) "MOVE_Walking" 0)
      (Transformation|DetachFromActor _returnvalue "KeepWorld" "KeepWorld" "KeepWorld"))))

(event Collision|EventHit
  (params (MyComp :type Primitive%20Component%20Object%20Reference) (Other :type Actor%20Object%20Reference) (OtherComp :type Primitive%20Component%20Object%20Reference) (bSelfMoved :type Boolean) (HitLocation :type Vector :default "0, 0, 0") (HitNormal :type Vector :default "0, 0, 0") (NormalImpulse :type Vector :default "0, 0, 0") (Hit :type Hit%20Result%20Structure%20%28by%20ref%29))
  (bind _returnvalue (Transformation|GetActorForwardVector Other))
  (bind _returnvalue_2 (Game|GetPlayerCharacter 0))
  (bind _returnvalue_3 (Game|GetPlayerCharacter 0))
  (bind (_x _y _z) (Math|Vector|BreakVector _returnvalue))
  (bind _mesh (Variables|/Script/Engine.Character|GetMesh _returnvalue_2))
  (if (== (Game|GetPlayerCharacter 0) Other)
    (if (> (Math|Vector|DotProduct _returnvalue HitNormal) 0.8)
      (Variables|Default|SetPushableDirection (Math|Vector|MakeVector (Math|Conversions|ToFloat(Integer) (Math|Float|Round _x)) (Math|Conversions|ToFloat(Integer) (Math|Float|Round _y)) (Math|Conversions|ToFloat(Integer) (Math|Float|Round _z))))
      (bind _canpush (CallFunction|CanPush))
      (if _canpush
        (Pawn|Components|CharacterMovement|DisableMovement (Variables|/Script/Engine.Character|GetCharacterMovement _returnvalue_3))
        (Transformation|AttachActorToActor _returnvalue_3 self "None" "KeepWorld" "KeepWorld" "KeepWorld" true)
        (if (Class|AnimInstance|IsAnyMontagePlaying (Components|SkeletalMesh|GetAnimInstance _mesh))
          (Utilities|FlowControl|Gate true :!label _label
            (:Exit
              (CallFunction|Push)))
          (else
            (Animation|Montage|PlayMontage _mesh "/Game/FreeSampleAnimationSet/Animations/PushSet/RootMotion/Heavy/01/MontagePush.MontagePush"
              (:OnNotifyBegin
                (CallFunction|Push)
                (goto _label Open)))))))))

(fn ConstructionScript)

(fn CanPush
  (bind _returnvalue (Game|GetPlayerCharacter 0))
  (bind _returnvalue_2 (Transformation|GetActorLocation))
  (bind _returnvalue_3 (Transformation|GetActorLocation _returnvalue))
  (bind (_outhit _returnvalue_4) (Collision|LineTraceByChannel _returnvalue_3 (+ _returnvalue_3 (* (Transformation|GetActorForwardVector _returnvalue) 1e+02)) "TraceTypeQuery1" false (Utilities|Array|MakeArray _returnvalue) "None" false))
  (if _returnvalue_4
    (if (== (.HitActor (Collision|BreakHitResult _outhit)) self)
      (bind _returnvalue_5 (Collision|BoxTraceByChannel (+ _returnvalue_2 (Math|Vector|MakeVector 0.0 0.0 1e+02)) (+ _returnvalue_2 (* (Variables|Default|GetPushableDirection) (Variables|Default|GetTravelDistance)) (Math|Vector|MakeVector 0.0 0.0 1e+02)) (* (.boxextent (StaticMesh|GetBounds (Variables|/Script/Engine.StaticMeshComponent|GetStaticMesh (Variables|Default|GetCube)))) (Variables|/Script/Engine.SceneComponent|GetRelativeScale3D (Variables|Default|GetCube)) "1.000000,1.000000,1.000000") "0, 0, 0" "TraceTypeQuery1" false 0 "None"))
      (return (not _returnvalue_5))
      (else
        (return false)))
    (else
      (return false))))