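; BP_Human is a player pawn with an item inventory and the ability to hand control to BP_Robot.
; BeginPlay creates the inventory widget, sizes the slot array and limits a scene capture to this actor; I toggles the widget.
; E sphere-traces low around the player, ignoring floors, then stacks or slots the BP_item, refreshes the widget and destroys the pickup.
; Left Alt, only when stationary, blends the camera to the robot, then possesses it.
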(event EventBeginPlay
  (Rendering|SceneCapture|ShowOnlyActorComponents (Variables|Default|GetSceneCaptureComponent2D) self false)
  (bind _returnvalue (UserInterface|CreateWidget "/Game/WIDGET/WB_inventaire.WB_inventaire_C"))
  (Variables|Default|Setinventaire _returnvalue)
  (Utilities|Array|Resize (Variables|Default|GetItem) 35)
  (Default|LoadInventaire (Variables|Default|Getinventaire) self)
  (bind _returnvalue_2 (Actor|GetActorOfClass "/Game/BLUEPRINTS/BP_Robot.BP_Robot_C"))
  (Variables|Default|SetRobot _returnvalue_2))

(event Collision|EventActorBeginOverlap
  (params (OtherActor :type Actor%20Object%20Reference)))

(event EventTick
  (params (DeltaSeconds :type Float%20%28single-precision%29)))

(event Input|KeyboardEvents|I
  (params (Key :type Key%20Structure :default "None"))
  (bind _returnvalue (Game|GetPlayerController 0))
  (bind _returnvalue_2 (Game|GetPlayerController 0))
  (:Pressed
    (if (Widget|IsVisible (Variables|Default|Getinventaire))
      (Widget|RemovefromParent (Variables|Default|Getinventaire))
      (Variables|/Script/Engine.PlayerController|SetbShowMouseCursor _returnvalue false)
      (Input|SetInputModeGameOnly _returnvalue false)
      (else
        (Variables|/Script/Engine.PlayerController|SetbShowMouseCursor _returnvalue_2 true)
        (Input|SetInputModeGameandUI _returnvalue_2 0 "DoNotLock" true false)
        (UserInterface|Viewport|AddtoViewport (Variables|Default|Getinventaire) 0)))))

(event Input|KeyboardEvents|E
  (params (Key :type Key%20Structure :default "None"))
  (bind _returnvalue (Game|GetPlayerCharacter 0))
  (bind _returnvalue_2 (Transformation|GetActorLocation _returnvalue))
  (bind _returnvalue_3 (- _returnvalue_2 "0.000000,0.000000,65.000000"))
  (:Pressed
    (bind _outactors (Actor|GetAllActorswithTag "floors"))
    (bind _outhit (Collision|SphereTraceByChannel _returnvalue_3 _returnvalue_3 1.2e+02 "TraceTypeQuery1" false _outactors "ForDuration"))
    (bind _asbp_item (Utilities|Casting|CastToBP_item (.HitActor (Collision|BreakHitResult _outhit))))
    (for (_array_element _array_index) (Variables|Default|GetItem)
      (Utilities|IsValid _asbp_item
        (:Is%20Valid
          (if (Math|Boolean|ANDBoolean (Utilities|Enum|Equal(Enum) (.Name (Utilities|Struct|BreakBP_structureinventaire _array_element)) (.Name (Utilities|Struct|BreakBP_structureinventaire (Variables|/Game/inventaire/objet/BP_item.BP_item_C|Getitem _asbp_item)))) (.Stackable (Utilities|Struct|BreakBP_structureinventaire (Variables|/Game/inventaire/objet/BP_item.BP_item_C|Getitem _asbp_item))) (<= (+ (.Quantity (Utilities|Struct|BreakBP_structureinventaire _array_element)) (.Quantity (Utilities|Struct|BreakBP_structureinventaire (Variables|/Game/inventaire/objet/BP_item.BP_item_C|Getitem _asbp_item)))) 64))
            (Utilities|Array|SetArrayElem (Variables|Default|GetItem) _array_index (Utilities|Struct|MakeBP_structureinventaire (.name (Variables|/Game/inventaire/objet/BP_item.BP_item_C|Getitem _asbp_item)) (.stackable (Variables|/Game/inventaire/objet/BP_item.BP_item_C|Getitem _asbp_item)) (+ (.Quantity (Utilities|Struct|BreakBP_structureinventaire _array_element)) (.Quantity (Utilities|Struct|BreakBP_structureinventaire (Variables|/Game/inventaire/objet/BP_item.BP_item_C|Getitem _asbp_item)))) (.thumnail (Variables|/Game/inventaire/objet/BP_item.BP_item_C|Getitem _asbp_item)) (.mesh (Variables|/Game/inventaire/objet/BP_item.BP_item_C|Getitem _asbp_item))))
            (Default|LoadInventaire (Variables|Default|Getinventaire) self :!label _label)
            (Actor|DestroyActor _asbp_item)
            (elif (== (.Quantity (Utilities|Struct|BreakBP_structureinventaire _array_element)) 0)
              (Utilities|Array|SetArrayElem (Variables|Default|GetItem) _array_index (Variables|/Game/inventaire/objet/BP_item.BP_item_C|Getitem _asbp_item))
              (goto _label))))))))

(event Input|KeyboardEvents|LeftAlt
  (params (Key :type Key%20Structure :default "None"))
  (bind _charactermovement (Variables|Character|GetCharacterMovement))
  (:Pressed
    (if (not (or (AI|Components|NavMovement|IsFalling _charactermovement) (> (Math|Vector|VectorLength (Variables|/Script/Engine.MovementComponent|GetVelocity _charactermovement)) 0.0)))
      (Game|Player|SetViewTargetwithBlend (Game|GetPlayerController 0) (Variables|Default|GetRobot) 0.7 "VTBlend_EaseInOut" 0.5 false)
      (Utilities|FlowControl|Delay 0.7)
      (Pawn|Possess (Game|GetPlayerController 0) (Variables|Default|GetRobot)))))

(fn ConstructionScript)