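; BP_Robot is a controllable robot character that lets the player switch control to BP_Human.
; On BeginPlay it caches the human and the robot's RobotAiController.
; Left Alt, only while neither falling nor moving, blends the camera to the human, possesses it after the blend delay, then returns the robot to its AI controller.
; The robot is looked up by class rather than self-reference, so it assumes a single instance.
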(event EventBeginPlay
  (bind _returnvalue (Actor|GetActorOfClass "/Game/BLUEPRINTS/BP_Human.BP_Human_C"))
  (Variables|Default|SetHuman _returnvalue)
  (bind _returnvalue_2 (Actor|GetActorOfClass "BP_Robot_C"))
  (bind _asrobot_ai_controller (Utilities|Casting|CastToRobotAiController (AI|GetAIController _returnvalue_2)))
  (Variables|Default|SetMonAiController _asrobot_ai_controller))

(event Collision|EventActorBeginOverlap
  (params (OtherActor :type Actor%20Object%20Reference)))

(event EventTick
  (params (DeltaSeconds :type Float%20%28single-precision%29)))

(event Input|KeyboardEvents|LeftAlt
  (params (Key :type Key%20Structure :default "None"))
  (bind _charactermovement (Variables|Character|GetCharacterMovement))
  (:Pressed
    (if (not (or (AI|Components|NavMovement|IsFalling _charactermovement) (> (Math|Vector|VectorLength (Variables|/Script/Engine.MovementComponent|GetVelocity _charactermovement)) 0.0)))
      (Game|Player|SetViewTargetwithBlend (Game|GetPlayerController 0) (Variables|Default|GetHuman) 0.7 "VTBlend_EaseInOut" 0.5 false)
      (Utilities|FlowControl|Delay 0.7)
      (Pawn|Possess (Game|GetPlayerController 0) (Variables|Default|GetHuman))
      (bind _returnvalue (Actor|GetActorOfClass "BP_Robot_C"))
      (Pawn|Possess (Variables|Default|GetMonAiController) _returnvalue))))

(fn ConstructionScript)