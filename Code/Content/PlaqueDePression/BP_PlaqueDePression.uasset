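; BP_PlaqueDePression is a pressure plate actor that drives a linked cable while a Character stands on it.
; Box overlap begin and end events, filtered by a Character cast, swap the plate mesh material and set IsFilling on LinkedCable to true or false.
; There is no occupant count, so any Character leaving stops the filling even if another remains.
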(event OnComponentBeginOverlap(Box)
  (params (OverlappedComponent :type Primitive%20Component%20Object%20Reference) (OtherActor :type Actor%20Object%20Reference) (OtherComp :type Primitive%20Component%20Object%20Reference) (OtherBodyIndex :type Integer) (bFromSweep :type Boolean) (SweepResult :type Hit%20Result%20Structure%20%28by%20ref%29))
  (bind _linkedcable (Variables|Default|GetLinkedCable))
  (Utilities|Casting|CastToCharacter OtherActor)
  (Rendering|Material|SetMaterial (Variables|Default|GetPlaqueDePressionMesh) 0 "/Engine/EditorMaterials/WidgetVertexColorMaterial.WidgetVertexColorMaterial")
  (Utilities|IsValid _linkedcable
    (:Is%20Valid
      (Variables|/Game/PlaqueDePression/BP_Cable.BP_Cable_C|SetIsFilling _linkedcable true))))

(event OnComponentEndOverlap(Box)
  (params (OverlappedComponent :type Primitive%20Component%20Object%20Reference) (OtherActor :type Actor%20Object%20Reference) (OtherComp :type Primitive%20Component%20Object%20Reference) (OtherBodyIndex :type Integer))
  (bind _linkedcable (Variables|Default|GetLinkedCable))
  (Utilities|Casting|CastToCharacter OtherActor)
  (Rendering|Material|SetMaterial (Variables|Default|GetPlaqueDePressionMesh) 0 "/Engine/VREditor/UI/ArrowMaterial.ArrowMaterial")
  (Utilities|IsValid _linkedcable
    (:Is%20Valid
      (Variables|/Game/PlaqueDePression/BP_Cable.BP_Cable_C|SetIsFilling _linkedcable false))))

(fn ConstructionScript)