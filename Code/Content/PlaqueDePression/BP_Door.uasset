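; BP_Door is a double sliding door that opens and closes through its Poweron and PowerOff events.
; Each event plays its own timeline from the start, linearly easing DoorRight and DoorLeft in opposite directions along local Y to open, or back to center to close.
; Because each timeline restarts from a fixed end position, interrupting a movement snaps the panels rather than reversing from their current position.
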(event EventPowerOff
  (bind _alpha (Timeline|Timeline_0 PlayFromStart)
    (:Update
      (Transformation|SetRelativeLocation (Variables|Default|GetDoorRight) (Math|Interpolation|Ease "Linear" _alpha "0.000000,200.000000,0.000000" "0.000000,0.000000,0.000000") false false)
      (Transformation|SetRelativeLocation (Variables|Default|GetDoorLeft) (Math|Interpolation|Ease "Linear" _alpha "0.000000,-200.000000,0.000000" "0.000000,0.000000,0.000000") false false))))

(event EventPoweron
  (bind _alpha (Timeline|OuverturePorte PlayFromStart)
    (:Update
      (Transformation|SetRelativeLocation (Variables|Default|GetDoorRight) (Math|Interpolation|Ease :Function "Linear" :Alpha _alpha :B "0.000000,200.000000,0.000000") false false)
      (Transformation|SetRelativeLocation (Variables|Default|GetDoorLeft) (Math|Interpolation|Ease :Function "Linear" :Alpha _alpha :B "0.000000,-200.000000,0.000000") false false))))

(fn ConstructionScript)